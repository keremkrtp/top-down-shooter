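; Spawner actor that endlessly creates BP_BasicAIFaster enemies around its own location, starting at BeginPlay.
; SpawnEnemy waits a random delay between MinSec and MaxSec, spawns the AI at a random reachable navigation point within a fixed radius, then calls itself to repeat.
; Spawns adjust for collisions but always happen, and the loop has no count limit or stop condition.
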(event Custom|SpawnEnemy
  (Utilities|FlowControl|Delay (Math|Random|RandomFloatinRange (Variables|Default|GetminSec) (Variables|Default|GetmaxSec)))
  (Game|SpawnActorfromClass "/Game/_BPs/AI/BP_BasicAIFaster.BP_BasicAIFaster_C" (Math|Conversions|ToTransform(Vector) (.RandomLocation (AI|Navigation|GetRandomReachablePointinRadius (Transformation|GetActorLocation) 3e+03 0 0))) "AdjustIfPossibleButAlwaysSpawn" "MultiplyWithRoot" 0 0)
  (CallFunction|SpawnEnemy))

(event EventBeginPlay
  (CallFunction|SpawnEnemy))

(fn ConstructionScript)
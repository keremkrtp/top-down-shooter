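; BP_BasicAIFaster is an enemy character that marches on the Nexus and diverts to the player when nearby.
; Tick updates its health bar widget and chooses the target, using SimpleMoveToActor until in attack range.
; Attacks play a montage and apply damage immediately, gated by a cooldown.
; Damage reduces health, and death grants the player gold regardless of the damage source, then destroys the actor.
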(event Custom|Event_Attack
  (params (Target :type Actor%20Object%20Reference))
  (if (Variables|Default|GetCanAttack)
    (Variables|Default|SetCanAttack false)
    (Animation|PlayAnimMontage "/Game/Characters/Mannequins/Anims/Unarmed/Attack/MM_Attack_01_Montage.MM_Attack_01_Montage" 1.0 "None")
    (Game|Damage|ApplyDamage Target (Variables|Default|GetAttackDamage) 0 0)
    (Utilities|FlowControl|Delay (Variables|Default|GetAttackCooldown))
    (Variables|Default|SetCanAttack true)))

(event EventBeginPlay
  (bind _outactors (Actor|GetAllActorswithTag "Nexus"))
  (Variables|Default|SetTargetNexus (Utilities|Array|Get(acopy) _outactors)))

(event Game|Damage|EventAnyDamage
  (params (Damage :type Float%20%28single-precision%29) (DamageType :type Damage%20Type%20Object%20Reference) (InstigatedBy :type Controller%20Object%20Reference) (DamageCauser :type Actor%20Object%20Reference))
  (Variables|Default|SetHealth (- (Variables|Default|GetHealth) Damage))
  (if (<= (Variables|Default|GetHealth) 0.0)
    (bind _asbp_player (Utilities|Casting|CastToBP_Player (Game|GetPlayerCharacter 0)))
    (Variables|/Game/_BPs/BP_Player.BP_Player_C|SetGold _asbp_player (+ (Variables|/Game/_BPs/BP_Player.BP_Player_C|GetGold _asbp_player) 20))
    (Actor|DestroyActor)
    (Development|PrintString "bot basicfaster öldü!! 20 GOLD KAZANDIN")))

(event EventTick
  (params (DeltaSeconds :type Float%20%28single-precision%29))
  (Utilities|FlowControl|Sequence
    (:then_0
      (bind _aswbp_enemy_health (Utilities|Casting|CastToWBP_EnemyHealth (UserInterface|GetUserWidgetObject (Variables|Default|GetHealthBarWidget))))
      (Progress|SetPercent (Variables|/Game/_BPs/UI/WBP_EnemyHealth.WBP_EnemyHealth_C|GetProgressBar_205 _aswbp_enemy_health) (/ (Variables|Default|GetHealth) (Variables|Default|GetMaxHealth))))
    (:then_1
      (if (< (Transformation|GetDistanceTo (Game|GetPlayerCharacter 0)) 8e+02)
        (if (< (Transformation|GetDistanceTo (Game|GetPlayerCharacter 0)) (Variables|Default|GetAttackRange))
          (CallFunction|EventAttack (Game|GetPlayerCharacter 0))
          (else
            (AI|Navigation|SimpleMovetoActor (Pawn|GetController) (Game|GetPlayerCharacter 0))))
        (elif (> (Transformation|GetDistanceTo (Variables|Default|GetTargetNexus)) (Variables|Default|GetAttackRange))
          (AI|Navigation|SimpleMovetoActor (Pawn|GetController) (Variables|Default|GetTargetNexus))
          (else
            (Components|Movement|StopMovementImmediately (Variables|Character|GetCharacterMovement))
            (CallFunction|EventAttack (Variables|Default|GetTargetNexus))))))))

(fn ConstructionScript)
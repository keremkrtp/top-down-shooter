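; BP_Turret is an auto-firing turret that uses AI sight perception to target actors tagged Enemy.
; Perception updates or a scan of known perceived actors set the target, and Tick rotates the head toward it, rescanning when none is valid.
; A looping timer spawns bullets from an arrow while targeting.
; Each shot spends ammo and updates a widget bar, and the turret destroys itself when ammo runs out.
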(event OnTargetPerceptionUpdated(AIPerception)
  (params (Actor :type Actor%20Object%20Reference) (Stimulus :type AI%20Stimulus%20Structure))
  (if (Actor|ActorHasTag Actor "Enemy")
    (Variables|Default|SetCurrentTarget Actor)
    (Variables|Default|SetHasTarget true)))

(event Custom|FireTurret
  (if (Variables|Default|GetHasTarget)
    (Game|SpawnActorfromClass "/Game/_BPs/GunSS/BP_Bullet.BP_Bullet_C" (Transformation|GetWorldTransform (Variables|Default|GetArrow)) "Undefined" "MultiplyWithRoot" self 0)
    (Variables|Default|SetAmmoCount (- (Variables|Default|GetAmmoCount) 1))
    (bind _aswbp_turretammo (Utilities|Casting|CastToWBP_Turretammo (UserInterface|GetUserWidgetObject (Variables|Default|GetAmmoWidget))))
    (Progress|SetPercent (Variables|/Game/_BPs/UI/WBP_Turretammo.WBP_Turretammo_C|GetAmmoBar _aswbp_turretammo) (/ (Math|Conversions|ToFloat(Integer) (Variables|Default|GetAmmoCount)) 1e+02))
    (if (<= (Variables|Default|GetAmmoCount) 0)
      (Actor|DestroyActor))))

(event EventTick
  (params (DeltaSeconds :type Float%20%28single-precision%29))
  (if (Variables|Default|GetHasTarget)
    (Utilities|IsValid (Variables|Default|GetCurrentTarget)
      (:Is%20Valid
        (Transformation|SetWorldRotation (Variables|Default|GetHead) (Math|Rotator|FindLookatRotation (Transformation|GetWorldLocation (Variables|Default|GetHead)) (Transformation|GetActorLocation (Variables|Default|GetCurrentTarget))) false false))
      (:Is%20Not%20Valid
        (CallFunction|FindBestTarget)))
    (else
      (CallFunction|FindBestTarget))))

(event EventBeginPlay
  (CallFunction|FindBestTarget)
  (Utilities|Time|SetTimerbyEvent (delegate Custom|FireTurret) 0.5 true)
  (CallFunction|FindBestTarget))

(fn ConstructionScript)

(fn FindBestTarget
  (Variables|Default|SetCurrentTarget 0)
  (Variables|Default|SetHasTarget false)
  (bind _array_element (Utilities|Array|ForEachLoopwithBreak (Class|AIPerceptionComponent|GetKnownPerceivedActors (Variables|Default|GetAIPerception) "/Script/AIModule.AISense_Sight") :!label _label)
    (:LoopBody
      (if (Actor|ActorHasTag _array_element "Enemy")
        (Utilities|IsValid _array_element
          (:Is%20Valid
            (Variables|Default|SetCurrentTarget _array_element)
            (Variables|Default|SetHasTarget true)
            (goto _label Break)))))))
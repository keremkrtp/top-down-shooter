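; BP_Nexus is a destructible base actor that doubles as the player's shop access point.
; Any damage lowers its health, shown each tick on a widget health bar; at zero it prints a message and destroys itself.
; A box overlap with BP_Player toggles the interact prompt and the actor's input.
; IA_Shop then opens WBP_Shop once, guarded by IsShopOpen, passing itself as owner, showing the cursor and playing a sound.
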(event OnComponentBeginOverlap(Box)
  (params (OverlappedComponent :type Primitive%20Component%20Object%20Reference) (OtherActor :type Actor%20Object%20Reference) (OtherComp :type Primitive%20Component%20Object%20Reference) (OtherBodyIndex :type Integer) (bFromSweep :type Boolean) (SweepResult :type Hit%20Result%20Structure%20%28by%20ref%29))
  (Utilities|Casting|CastToBP_Player OtherActor)
  (Rendering|SetVisibility (Variables|Default|GetInteractPrompt) true false)
  (Input|EnableInput (Game|GetPlayerController 0)))

(event OnComponentEndOverlap(Box)
  (params (OverlappedComponent :type Primitive%20Component%20Object%20Reference) (OtherActor :type Actor%20Object%20Reference) (OtherComp :type Primitive%20Component%20Object%20Reference) (OtherBodyIndex :type Integer))
  (Utilities|Casting|CastToBP_Player OtherActor)
  (Rendering|SetVisibility (Variables|Default|GetInteractPrompt) false false)
  (Input|DisableInput (Game|GetPlayerController 0)))

(event Input|EnhancedActionEvents|EnhancedInputActionIA_Shop
  (params (ActionValue :type Boolean) (ElapsedSeconds :type Float%20%28double-precision%29) (TriggeredSeconds :type Float%20%28double-precision%29) (InputAction :type Input%20Action%20Object%20Reference :default "/Game/Input/IA_Shop.IA_Shop"))
  (:Started
    (if (not (Variables|Default|GetisShopOpen?))
      (Variables|Default|SetisShopOpen? true)
      (bind _returnvalue (UserInterface|CreateWidget "/Game/_BPs/UI/WBP_Shop.WBP_Shop_C" 0 self))
      (UserInterface|Viewport|AddtoViewport _returnvalue 0)
      (Variables|/Script/Engine.PlayerController|SetbShowMouseCursor (Game|GetPlayerController 0) true)
      (Audio|PlaySound2D "/Game/_SOUNDS/cash-register-fake-88639.cash-register-fake-88639" 1.0 1.0 0.0 0 0))))

(event Game|Damage|EventAnyDamage
  (params (Damage :type Float%20%28single-precision%29) (DamageType :type Damage%20Type%20Object%20Reference) (InstigatedBy :type Controller%20Object%20Reference) (DamageCauser :type Actor%20Object%20Reference))
  (Variables|Default|SetHealth (- (Variables|Default|GetHealth) Damage))
  (if (<= (Variables|Default|GetHealth) 0.0)
    (Development|PrintString "Merkez yıkıldı reis")
    (Actor|DestroyActor)))

(event EventTick
  (params (DeltaSeconds :type Float%20%28single-precision%29))
  (Utilities|FlowControl|Sequence
    (:then_0
      (bind _aswbp_enemy_health (Utilities|Casting|CastToWBP_EnemyHealth (UserInterface|GetUserWidgetObject (Variables|Default|GetHealthBar))))
      (Progress|SetPercent (Variables|/Game/_BPs/UI/WBP_EnemyHealth.WBP_EnemyHealth_C|GetProgressBar_205 _aswbp_enemy_health) (/ (Variables|Default|GetHealth) (Variables|Default|GetMaxHealth))))))

(fn ConstructionScript)
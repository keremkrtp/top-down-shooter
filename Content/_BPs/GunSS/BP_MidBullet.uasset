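; BP_MidBullet is a bullet projectile actor that deals a fixed amount of damage to whatever its collision sphere hits.
; On BeginPlay the sphere is set to ignore its owner, the BP_Nexus actor and the player character while moving.
; On hit it applies damage, plays an attenuated impact sound, spawns a small steam particle effect at the hit location, then destroys itself.
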(event OnComponentHit(Sphere)
  (params (HitComponent :type Primitive%20Component%20Object%20Reference) (OtherActor :type Actor%20Object%20Reference) (OtherComp :type Primitive%20Component%20Object%20Reference) (NormalImpulse :type Vector :default "0, 0, 0") (Hit :type Hit%20Result%20Structure%20%28by%20ref%29))
  (bind _location (Collision|BreakHitResult Hit))
  (Game|Damage|ApplyDamage OtherActor 1e+01 0 0)
  (Audio|PlaySoundatLocation "/Game/_SOUNDS/bulletimpact2-442718.bulletimpact2-442718" _location "0, 0, 0" 1.0 1.0 0.0 "/Game/_SOUNDS/SA_AmmoSound.SA_AmmoSound" 0 0 0)
  (Effects|SpawnEmitteratLocation "/Game/StarterContent/Particles/P_Steam_Lit.P_Steam_Lit" _location "0, 0, 0" "0.200000,0.200000,0.200000")
  (Actor|DestroyActor))

(event EventBeginPlay
  (Collision|IgnoreActorwhenMoving (Variables|Default|GetSphere) (Components|GetOwner) true)
  (bind _returnvalue (Actor|GetActorOfClass "/Game/_BPs/nexus/BP_Nexus.BP_Nexus_C"))
  (Collision|IgnoreActorwhenMoving (Variables|Default|GetSphere) _returnvalue true)
  (Collision|IgnoreActorwhenMoving (Variables|Default|GetSphere) (Game|GetPlayerCharacter 0) true))

(fn ConstructionScript)